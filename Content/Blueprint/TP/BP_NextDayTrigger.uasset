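; BP_NextDayTrigger is a trigger volume that shows the Go_nextDay widget while the player is inside it.
; When MyPlayer begins overlapping TriggerBox, it creates and stores the widget, adds it to the viewport, shows the mouse cursor and switches to UI-only input.
; When the overlap ends, it removes the widget after a validity check, hides the cursor and restores game-only input.
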(event OnComponentBeginOverlap(TriggerBox)
  (params (OverlappedComponent :type Primitive%20Component%20Object%20Reference) (OtherActor :type Actor%20Object%20Reference) (OtherComp :type Primitive%20Component%20Object%20Reference) (OtherBodyIndex :type Integer) (bFromSweep :type Boolean) (SweepResult :type Hit%20Result%20Structure%20%28by%20ref%29))
  (bind _returnvalue (Game|GetPlayerController 0))
  (Utilities|Casting|CastToMyPlayer OtherActor)
  (bind _returnvalue_2 (UserInterface|CreateWidget "/Game/UMG/Go_nextDay.Go_nextDay_C"))
  (UserInterface|Viewport|AddtoViewport _returnvalue_2 0)
  (Variables|Default|SetGonextDayvariable _returnvalue_2)
  (Variables|/Script/Engine.PlayerController|SetbShowMouseCursor _returnvalue true)
  (Input|SetInputModeUIOnly _returnvalue 0 "DoNotLock" false))

(event OnComponentEndOverlap(TriggerBox)
  (params (OverlappedComponent :type Primitive%20Component%20Object%20Reference) (OtherActor :type Actor%20Object%20Reference) (OtherComp :type Primitive%20Component%20Object%20Reference) (OtherBodyIndex :type Integer))
  (bind _returnvalue (Game|GetPlayerController 0))
  (Utilities|Casting|CastToMyPlayer OtherActor)
  (Utilities|IsValid 0
    (:Is%20Valid
      (Widget|RemovefromParent (Variables|Default|GetGonextDayvariable)))
    (:Is%20Not%20Valid
      _))
  (Variables|/Script/Engine.PlayerController|SetbShowMouseCursor _returnvalue false)
  (Input|SetInputModeGameOnly _returnvalue false))

(event EventBeginPlay)

(event Collision|EventActorBeginOverlap
  (params (OtherActor :type Actor%20Object%20Reference)))

(event EventTick
  (params (DeltaSeconds :type Float%20%28single-precision%29)))

(fn ConstructionScript)