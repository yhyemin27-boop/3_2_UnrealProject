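; BP_FinalProjectGameMode is a game mode that handles evidence submission in NPC conversations.
; SubmitEvidence builds a DT_DialogueResponse row name from the game instance's current day and NPC ID plus the evidence ID.
; If the row's required evidence matches, it shows the success dialogue in the chat widget, with no failure response.
; HideChatWidget removes that widget and clears its reference; the widget is never created here.
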(event EventBeginPlay)

(event EventTick
  (params (DeltaSeconds :type Float%20%28single-precision%29)))

(fn ConstructionScript)

(fn SubmitEvidence
  (params (Evidence_ID :type Evidence%20Data%20Structure))
  (bind _evidenceid (Utilities|Struct|BreakEvidenceData Evidence_ID))
  (bind _chattingwidgetref (Variables|Default|GetChattingWidgetRef))
  (bind _asbp_game_instance (Utilities|Casting|CastToBP_GameInstance (Game|GetGameInstance)))
  (bind _returnvalue (Utilities|GetDataTableRow "/Game/MPC/DT_DialogueResponse.DT_DialogueResponse" (Utilities|String|StringToName (Utilities|String|Append "Day_" (Utilities|String|ToString(Integer) (Variables|/Script/finalproject.My_GameInstance|GetCurrentDay _asbp_game_instance)) "_" (Utilities|String|ToString(Name) (Variables|/Script/finalproject.My_GameInstance|GetCurrentNPCID _asbp_game_instance)) "_" (Utilities|String|ToString(Name) _evidenceid))))
    (:then
      (if (== (.Required_Evidence_ID (Utilities|Struct|BreakDialogueResponseData _returnvalue)) _evidenceid)
        (Default|SetCurrentText _chattingwidgetref (.Success_Dialogue (Utilities|Struct|BreakDialogueResponseData _returnvalue)))
        (UserInterface|Viewport|AddtoViewport _chattingwidgetref 0)))))

(fn HideChatWidget
  (Utilities|IsValid (Variables|Default|GetChattingWidgetRef)
    (:Is%20Valid
      (Widget|RemovefromParent (Variables|Default|GetChattingWidgetRef))
      (Variables|Default|SetChattingWidgetRef 0))))