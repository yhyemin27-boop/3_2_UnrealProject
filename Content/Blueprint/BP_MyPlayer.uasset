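; Player Blueprint for an evidence-gathering game, managing the inventory, note and start-screen UI.
; BeginPlay creates the Start, Force, note and inventory widgets, plays a start sound and sets UI-only input focused on the start screen.
; Inventory and note input actions toggle widget visibility and the cursor in game-only input mode, both writing IsInventoryOpen.
; OnEvidenceFound adds evidence to a list and passes it with the returned index to the inventory widget.
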(event Input|EnhancedActionEvents|EnhancedInputActionIA_Note
  (params (ActionValue :type Boolean) (ElapsedSeconds :type Float%20%28double-precision%29) (TriggeredSeconds :type Float%20%28double-precision%29) (InputAction :type Input%20Action%20Object%20Reference :default "/Game/Input/Actions/IA_Note.IA_Note"))
  (bind _returnvalue (Game|GetPlayerController 0))
  (:Completed
    (if (Variables|Default|GetIsNoteWidgetRef)
      (Variables|/Script/UMG.Widget|SetVisibility (Variables|Default|GetNoteWidgetRef) "Collapsed")
      (Input|SetInputModeGameOnly _returnvalue false)
      (Variables|/Script/Engine.PlayerController|SetbShowMouseCursor _returnvalue false)
      (Variables|Default|SetIsInventoryOpen false)
      (Variables|Default|SetNoteWidgetRef (Variables|Default|GetNoteWidgetRef))
      (Variables|Default|SetIsNoteWidgetRef false)
      (else
        (Variables|Default|SetNoteWidgetRef (Variables|Default|GetNoteWidgetRef))
        (Variables|Default|SetIsNoteWidgetRef true)
        (Variables|/Script/UMG.Widget|SetVisibility (Variables|Default|GetNoteWidgetRef) "Visible")
        (Input|SetInputModeGameOnly _returnvalue false)
        (Variables|/Script/Engine.PlayerController|SetbShowMouseCursor _returnvalue true)
        (Variables|Default|SetIsInventoryOpen true)))))

(event Input|EnhancedActionEvents|EnhancedInputActionIA_Inventory
  (params (ActionValue :type Boolean) (ElapsedSeconds :type Float%20%28double-precision%29) (TriggeredSeconds :type Float%20%28double-precision%29) (InputAction :type Input%20Action%20Object%20Reference :default "/Game/Input/Actions/IA_Inventory.IA_Inventory"))
  (bind _returnvalue (Game|GetPlayerController 0))
  (:Completed
    (if (Variables|Default|GetIsInventoryOpen)
      (Variables|/Script/UMG.Widget|SetVisibility (Variables|Default|GetInventoryWidgetRef) "Hidden")
      (Variables|Default|SetInventoryWidgetRef (Variables|Default|GetInventoryWidgetRef))
      (Input|SetInputModeGameOnly _returnvalue false)
      (Variables|/Script/Engine.PlayerController|SetbShowMouseCursor _returnvalue false)
      (Variables|Default|SetIsInventoryOpen false)
      (else
        (Variables|Default|SetInventoryWidgetRef (Variables|Default|GetInventoryWidgetRef))
        (Variables|/Script/UMG.Widget|SetVisibility (Variables|Default|GetInventoryWidgetRef) "Visible")
        (Input|SetInputModeGameOnly _returnvalue false)
        (Variables|/Script/Engine.PlayerController|SetbShowMouseCursor _returnvalue true)
        (Variables|Default|SetIsInventoryOpen true)))))

(event Collision|EventActorBeginOverlap
  (params (OtherActor :type Actor%20Object%20Reference)))

(event EventBeginPlay
  (bind _returnvalue (Game|GetPlayerController 0))
  (bind _returnvalue_2 (Game|GetPlayerController 0))
  (bind _returnvalue_3 (UserInterface|CreateWidget "/Game/UMG/start.start_C" _returnvalue_2))
  (bind _returnvalue_4 (UserInterface|CreateWidget "/Game/UMG/force.force_C" _returnvalue_2))
  (bind _returnvalue_5 (UserInterface|CreateWidget "/Game/UMG/Notewidget.Notewidget_C" _returnvalue_2))
  (UserInterface|Viewport|AddtoViewport _returnvalue_5 0)
  (Variables|/Script/UMG.Widget|SetVisibility _returnvalue_5 "Visible")
  (Variables|Default|SetNoteWidgetRef _returnvalue_5)
  (bind _returnvalue_6 (UserInterface|CreateWidget "/Game/UMG/UMG_Inventory.UMG_Inventory_C" _returnvalue_2))
  (UserInterface|Viewport|AddtoViewport _returnvalue_6 0)
  (Variables|/Script/UMG.Widget|SetVisibility _returnvalue_6 "Collapsed")
  (Variables|Default|SetInventoryWidgetRef _returnvalue_6)
  (Variables|/Game/UMG/start.start_C|SetstartWidgetRef _returnvalue_3 _returnvalue_3)
  (UserInterface|Viewport|AddtoViewport _returnvalue_3 0)
  (Input|SetInputModeUIOnly _returnvalue _returnvalue_3 "DoNotLock" false)
  (Variables|/Script/Engine.PlayerController|SetbShowMouseCursor _returnvalue true)
  (bind _returnvalue_7 (Audio|SpawnSound2D "/Game/SOUND/START/start.start" 1.0 1.0 0.0 0))
  (Variables|Default|SetSound_1 _returnvalue_7))

(event EventOnEvidenceFound
  (params (EvidenceData :type Evidence%20Data%20Structure%20%28by%20ref%29))
  (bind _returnvalue (Class|MyPlayer|AddEvidencetoEvidenceList EvidenceData))
  (Default|SetItemData (Variables|Default|GetInventoryWidgetRef) EvidenceData _returnvalue))

(fn ConstructionScript)

(fn OpenInventory
  (params (EvidenceList :type Array%20of%20Evidence%20Data%20Structures))
  (bind _returnvalue (UserInterface|CreateWidget "/Game/UMG/UMG_Inventory.UMG_Inventory_C" (Game|GetPlayerController 0)))
  (bind _output_get (Variables|Default|SetInventoryWidgetRef _returnvalue))
  (UserInterface|Viewport|AddtoViewport _output_get 0))