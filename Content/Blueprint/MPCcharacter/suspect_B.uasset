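; Suspect B Blueprint that opens a suspect chat screen when its dialogue-initiated event fires.
; It gets or creates the WDB_suspect_chating widget, caching the reference on BP_FinalProjectGameMode for reuse.
; It then passes in the dialogue text, adds the widget to the viewport and switches the first player controller to UI-only input.
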(event EventBeginPlay)

(event Collision|EventActorBeginOverlap
  (params (OtherActor :type Actor%20Object%20Reference)))

(event EventTick
  (params (DeltaSeconds :type Float%20%28single-precision%29)))

(event EventOnDialogueInitiated
  (params (DialogueText :type Text%20%28by%20ref%29))
  (bind _asbp_final_project_game_mode (Utilities|Casting|CastToBP_FinalProjectGameMode (Game|GetGameMode)))
  (Utilities|IsValid (Variables|/Game/Blueprint/BP_FinalProjectGameMode.BP_FinalProjectGameMode_C|GetChattingWidgetRef _asbp_final_project_game_mode)
    (:Is%20Valid
      _)
    (:Is%20Not%20Valid
      (bind _returnvalue (UserInterface|CreateWidget "/Game/UMG/WDB_suspect_chating.WDB_suspect_chating_C" (Game|GetPlayerController 0)))
      (bind _output_get (Variables|/Game/Blueprint/BP_FinalProjectGameMode.BP_FinalProjectGameMode_C|SetChattingWidgetRef _asbp_final_project_game_mode _returnvalue))))
  (Default|SetCurrentText (Variables|/Game/Blueprint/BP_FinalProjectGameMode.BP_FinalProjectGameMode_C|GetChattingWidgetRef _asbp_final_project_game_mode) DialogueText)
  (UserInterface|Viewport|AddtoViewport (Variables|/Game/Blueprint/BP_FinalProjectGameMode.BP_FinalProjectGameMode_C|GetChattingWidgetRef _asbp_final_project_game_mode) 0)
  (Input|SetInputModeUIOnly (Game|GetPlayerController 0) 0 "DoNotLock" false))

(fn ConstructionScript)